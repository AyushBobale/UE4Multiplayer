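; Player controller for a multiplayer lobby tag game, handling local input, UI and chat.
; It creates chat, scoreboard, countdown, info and win-screen widgets, switching input mode when chat takes focus.
; Left click fires the character's tag only for GS_Lobby's TagOwner; chat sends and the T-key countdown go through GM_Lobby.
; Events also freeze or unfreeze pawn input and destroy the session to return to the menu.
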(event Custom|ShowCountDown
  ;[1 1 1] Countdown
  (bind _returnvalue (UserInterface|CreateWidget "/Game/Games/Casual_Lobby/Blueprints/W_CountDown.W_CountDown_C"))
  (UserInterface|Viewport|AddtoViewport _returnvalue 0))

(event Custom|Unfreeze
  ;[1 1 1] Enable input
  (Input|EnableInput (Pawn|GetControlledPawn) self)
  (Development|PrintString "Enabled Input"))

(event Custom|ShowInfo
  ;[1 1 1] Show info widget
  (bind _returnvalue (UserInterface|CreateWidget "/Game/Games/Casual_Lobby/Blueprints/W_info.W_info_C"))
  (UserInterface|Viewport|AddtoViewport _returnvalue 0))

(event Custom|Freeze
  ;[1 1 1] Disable Input
  (Input|DisableInput (Pawn|GetControlledPawn) self))

(event Custom|ShowWinnerWidget
  (params (won :type Boolean))
  ;[1 1 1] Removes all widget and adds the win screens
  (Viewport|RemoveAllWidgets)
  (bind _returnvalue (UserInterface|CreateWidget "/Game/Games/Casual_Lobby/Blueprints/W_WinScreen.W_WinScreen_C" 0 won))
  (UserInterface|Viewport|AddtoViewport _returnvalue 0))

(event Custom|BackToMainMenu
  ;[1 1 1] Quitting to mainmenu
  (|DestroySession self
    (:OnSuccess
      (Development|PrintString "SessionDestroyed")
      (Game|OpenLevel(byObjectReference) "/Game/Maps/MAP_MultiplayerMenu.MAP_MultiplayerMenu"))
    (:OnFailure
      (Development|PrintString "SessionWas not destroyed"))))

(event Custom|CreateChatWidget
  ;[1 1 1] Create chat widget
  (bind _returnvalue (UserInterface|CreateWidget "/Game/Games/Casual_Lobby/Blueprints/W_Chat.W_Chat_C"))
  (bind _output_get (Variables|Default|SetW_Chat _returnvalue))
  (UserInterface|Viewport|AddtoViewport _output_get 0))

(event Custom|ShowChatWidget
  (params (focused :type Boolean))
  (bind _self self)
  ;[1 1 1] Show chat widget
  (Default|SetFocusonChat (Variables|Default|GetW_Chat) focused)
  (if focused
    (Input|SetInputModeGameandUI _self (Variables|Default|GetW_Chat) "DoNotLock" true)
    (else
      (Input|SetInputModeGameOnly _self))))

(event Custom|ServerSendMessage
  (params (Sender :type String) (Message :type String))
  ;[1 1 1] chat system
  (bind _asgm_lobby (Utilities|Casting|CastToGM_Lobby (Game|GetGameMode)))
  (Default|SendMessagetoEveryone _asgm_lobby Sender Message))

(event Custom|AddMessageToChat
  (params (Sender :type String) (Message :type String))
  ;[1 1 1] chat system
  (Default|AddMessageOntoMessageList (Variables|Default|GetW_Chat) Sender Message))

(event EventBeginPlay
  ;[1 1 1] Seting game state
  (Input|SetInputModeGameOnly self)
  (bind _asgs_lobby (Utilities|Casting|CastToGS_Lobby (Game|GetGameState)))
  (Variables|Default|SetGS_Lobby _asgs_lobby)
  (CallFunction|CreateChatWidget))

(event EventTick
  (params (DeltaSeconds :type Float%20%28single-precision%29)))

(event Input|MouseEvents|LeftMouseButton
  (params (Key :type Key%20Structure :default "None"))
  ;[1 1 1] Shooting Tags
  (:Pressed
    (if (== (Variables|/Game/Games/Casual_Lobby/Blueprints/GS_Lobby.GS_Lobby_C|GetTagOwner (Variables|Default|GetGS_Lobby)) self)
      (bind _asthird_person_character (Utilities|Casting|CastToThirdPersonCharacter (Pawn|GetControlledPawn)))
      (Default|ShootTag _asthird_person_character))))

(event Input|KeyboardEvents|Tab
  (params (Key :type Key%20Structure :default "None"))
  ;[1 1 1] showing ScoreBoard
  (:Pressed
    (bind _returnvalue (UserInterface|CreateWidget "/Game/Games/Casual_Lobby/Blueprints/W_ScoreBoard.W_ScoreBoard_C"))
    (bind _output_get (Variables|Default|SetScoreBoard _returnvalue))
    (UserInterface|Viewport|AddtoViewport _output_get 0))
  (:Released
    (Widget|RemovefromParent (Variables|Default|GetScoreBoard))))

(event Input|KeyboardEvents|T
  (params (Key :type Key%20Structure :default "None"))
  ;[1 1 1] Start countdown
  (:Pressed
    (bind _asgm_lobby (Utilities|Casting|CastToGM_Lobby (Game|GetGameMode)))
    (Default|CountDown _asgm_lobby)))

(event Input|KeyboardEvents|Enter
  (params (Key :type Key%20Structure :default "None"))
  ;[1 1 1] Show chat widget
  (:Pressed
    (CallFunction|ShowChatWidget true)))

(fn ConstructionScript)