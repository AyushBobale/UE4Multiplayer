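; Lobby game mode that runs a timed tag match, where the player with the fewest points wins.
; PostLogin spawns and possesses a named character per player and alternates them between teams A and B.
; After a countdown, a random player gets the tag, and a looping one-second timer adds points to the current owner.
; At time-out it freezes players, shows results and returns them to the main menu; it also relays chat.
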(event Custom|CountDown
  ;[1 1 1] Show CountDown
  (if (not (Variables|Default|Getstarted))
    (for _array_element (Variables|Default|Getplayers)
      (Default|ShowCountDown _array_element))
    (Variables|Default|Setstarted true)
    (Utilities|FlowControl|Delay 5.0)
    (CallFunction|Unfreeze)))

(event Custom|Unfreeze
  ;[1 1 1] Enabling input
  (for _array_element (Variables|Default|Getplayers)
    (Default|Unfreeze _array_element))
  ;[1 1 1] Counter
  (Variables|/Game/Games/Casual_Lobby/Blueprints/GS_Lobby.GS_Lobby_C|SetcurrentTime (Variables|Default|GetGS_Lobby) (Variables|Default|GetmatchTime))
  (bind _returnvalue (Utilities|Time|SetTimerbyEvent (delegate Custom|Count) 1.0 true))
  (CallFunction|ShowTimer)
  (CallFunction|ChooseRandomTagOwner))

(event Custom|Count
  ;[1 1 1] Counter
  (bind _result (Math|Integer|DecrementInt (Variables|/Game/Games/Casual_Lobby/Blueprints/GS_Lobby.GS_Lobby_C|GetcurrentTime (Variables|Default|GetGS_Lobby)))
    (:%20%20
      (Math|Integer|IncrementInt (Variables|/Game/Games/Casual_Lobby/Blueprints/PS_Lobby.PS_Lobby_C|GetPoints (.AsPS%20Lobby (Utilities|Casting|CastToPS_Lobby (Variables|/Script/Engine.Controller|GetPlayerState (Variables|/Game/Games/Casual_Lobby/Blueprints/GS_Lobby.GS_Lobby_C|GetTagOwner (Variables|Default|GetGS_Lobby))))))
        (:%20%20
          (if (== _result 0)
            (Utilities|Time|PauseTimerbyHandle (stale Custom|Unfreeze _returnvalue))
            (CallFunction|Freeze)
            (CallFunction|CheckPoints)
            (Utilities|FlowControl|Delay 3.0)
            (CallFunction|BacktoMainMenu)))))))

(event Custom|ShowTimer
  ;[1 1 1] Show Info widget
  (for _array_element (Variables|Default|Getplayers)
    (Default|ShowInfo _array_element)))

(event Custom|Freeze
  ;[1 1 1] Disable input
  (for _array_element (Variables|Default|Getplayers)
    (Default|Freeze _array_element)))

(event Custom|SwitchOwner
  (params (TagOwner :type PC%20Lobby%20Object%20Reference))
  ;[1 1 1] Switching tags
  (Variables|/Game/Games/Casual_Lobby/Blueprints/GS_Lobby.GS_Lobby_C|SetTagOwner (Variables|Default|GetGS_Lobby) TagOwner))

(event Custom|ChooseRandomTagOwner
  ;[1 1 1] Seleting random player with tag
  (Variables|/Game/Games/Casual_Lobby/Blueprints/GS_Lobby.GS_Lobby_C|SetTagOwner (Variables|Default|GetGS_Lobby) (Utilities|Array|Get(acopy) (Variables|Default|Getplayers) (Math|Random|RandomIntegerinRange 0 (- (Utilities|Array|Length (Variables|Default|Getplayers)) 1)))))

(event Custom|CheckPoints
  ;[1 1 1] Checking for winners
  (for _array_element (Variables|Default|Getplayers)
    (Utilities|IsValid (Variables|Default|GetWinner)
      (:Is%20Valid
        (if (< (Variables|/Game/Games/Casual_Lobby/Blueprints/PS_Lobby.PS_Lobby_C|GetPoints (.AsPS%20Lobby (Utilities|Casting|CastToPS_Lobby (Variables|/Script/Engine.Controller|GetPlayerState _array_element)))) (Variables|/Game/Games/Casual_Lobby/Blueprints/PS_Lobby.PS_Lobby_C|GetPoints (.AsPS%20Lobby (Utilities|Casting|CastToPS_Lobby (Variables|/Script/Engine.Controller|GetPlayerState (Variables|Default|GetWinner))))))
          (Variables|Default|SetWinner _array_element)))
      (:Is%20Not%20Valid
        (Variables|Default|SetWinner _array_element))))
  ;[1 1 1] Show winner widget
  (Default|ShowWinnerWidget (Variables|Default|GetWinner) true)
  (for _array_element_2 (Variables|Default|Getplayers)
    (if (!= _array_element_2 (Variables|Default|GetWinner))
      (Default|ShowWinnerWidget _array_element_2 false))))

(event Custom|BackToMainMenu
  ;[1 1 1] Quitting to main menu
  (for _array_element (Variables|Default|Getplayers)
    (Default|BacktoMainMenu _array_element)))

(event Custom|SendMessageToEveryone
  (params (Sender :type String) (Message :type String))
  ;[1 1 1] Chat System
  (for _array_element (Variables|Default|Getplayers)
    (Default|AddMessagetoChat _array_element Sender Message)))

(event EventBeginPlay
  ;[1 1 1] Saving Game state
)

(event EventTick
  (params (DeltaSeconds :type Float%20%28single-precision%29)))

(event EventPostLogin
  (params (NewPlayer :type Player%20Controller%20Object%20Reference))
  (bind _players (Variables|Default|Getplayers))
  (bind _playerstate (Variables|/Script/Engine.Controller|GetPlayerState NewPlayer))
  (bind _returnvalue (Utilities|Array|Length _players))
  (bind _returnvalue_2 (PlayerState|GetPlayerName _playerstate))
  (bind _returnvalue_3 (- _returnvalue 1))
  (bind _returnvalue_4 (Math|Integer|%(Integer) _returnvalue_3 2))
  (bind _returnvalue_5 (== _returnvalue_4 0))
  ;[1 1 1] Adding Plyrs
  (bind _aspc_lobby (Utilities|Casting|CastToPC_Lobby NewPlayer))
  (Utilities|Array|Add (Variables|Default|Getplayers) _aspc_lobby)
  (bind _returnvalue_6 (Game|SpawnActorfromClass "/Game/ThirdPersonBP/Blueprints/ThirdPersonCharacter.ThirdPersonCharacter_C" (Transformation|GetActorTransform (Class|GameModeBase|FindPlayerStart NewPlayer (Utilities|String|ToString(Integer) (- (Utilities|Array|Length (Variables|Default|Getplayers)) 1)))) "Undefined" 0 (PlayerState|GetPlayerName (Variables|/Script/Engine.Controller|GetPlayerState NewPlayer)) 0))
  (Pawn|Possess NewPlayer _returnvalue_6)
  (bind _asgs_lobby (Utilities|Casting|CastToGS_Lobby (Game|GetGameState)))
  (Variables|Default|SetGS_Lobby _asgs_lobby)
  (if _returnvalue_5
    (Utilities|Array|Add (Variables|/Game/Games/Casual_Lobby/Blueprints/GS_Lobby.GS_Lobby_C|GetTeamA (Variables|Default|GetGS_Lobby)) _returnvalue_2)
    (else
      (Utilities|Array|Add (Variables|/Game/Games/Casual_Lobby/Blueprints/GS_Lobby.GS_Lobby_C|GetTeamB (Variables|Default|GetGS_Lobby)) _returnvalue_2)))
  (bind _asps_lobby (Utilities|Casting|CastToPS_Lobby (Variables|/Script/Engine.Controller|GetPlayerState NewPlayer)))
  (Variables|/Game/Games/Casual_Lobby/Blueprints/PS_Lobby.PS_Lobby_C|SetTeam _asps_lobby (Utilities|String|SelectString "A" "B" _returnvalue_5)))

(fn ConstructionScript)